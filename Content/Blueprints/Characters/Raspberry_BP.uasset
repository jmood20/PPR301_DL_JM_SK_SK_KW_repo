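; Raspberry player character with replicated health and a limited bomb supply, both initialized on the server at BeginPlay.
; R calls a server event that spawns a Bullet_Asset in front of the character and decrements the count; Space plays a jump sound.
; Damage applies on authority; at zero health it resets health, shows the game-over widget, pauses and destroys the actor.
; RepNotify functions refresh the HP and bomb-count text.
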(event Custom|ServerAttemptSpwanBomb
  (CallFunction|AttemptSpawnBomb))

(event EventBeginPlay
  ;[1 1 1] Initalize character attributes only on the server
  (Networking|SwitchHasAuthority
    (:Authority
      (CallFunction|InitAttributes))))

(event Game|Damage|EventAnyDamage
  (params (Damage :type Float%20%28single-precision%29) (DamageType :type Damage%20Type%20Object%20Reference) (InstigatedBy :type Controller%20Object%20Reference) (DamageCauser :type Actor%20Object%20Reference))
  ;[0 0.1098 1] Handle Damage
  (CallFunction|OnTakeDamage Damage))

(event Input|KeyboardEvents|SpaceBar
  (params (Key :type Key%20Structure))
  ;[1 1 1] Jump Sound
  (:Pressed
    (Audio|PlaySound2D "/Game/Sounds/Jump.Jump" 1.0 1.0 0.0 0 0)))

(event Input|KeyboardEvents|R
  (params (Key :type Key%20Structure))
  ;[1 1 1] Attempt to Spawn a Bomb on RMB
  (:Pressed
    (bind _hasbombsremaining (CallFunction|HasBombs))
    (if _hasbombsremaining
      (CallFunction|ServerAttemptSpwanBomb))))

(fn ConstructionScript
  (|CallParentFunction))

(fn InitAttributes
  (Networking|SwitchHasAuthority
    (:Authority
      (CallFunction|InitHealth)
      (CallFunction|InitBombs))))

(fn InitHealth
  (Variables|Attributes|SetHealth (Variables|Attributes|GetMaxHealth)))

(fn InitBombs
  (Variables|Attributes|SetBombCount (Variables|Attributes|GetMaxBombCount)))

(fn OnRepBombCount
  (CallFunction|UpdateCharcaterDisplayText))

(fn OnRepHealth
  (CallFunction|UpdateCharcaterDisplayText))

(fn UpdateCharcaterDisplayText
  (Rendering|Components|TextRender|SetText (LocalVariables|GetNewLocalVar_0) (Utilities|Text|ToText(String) (Utilities|String|BuildString(Integer) (Utilities|String|BuildString(Float) "" "HP: " (Variables|Attributes|GetHealth) " Bomb Count: ") "" (Variables|Attributes|GetBombCount)))))

(fn OnTakeDamage
  (params (Damage :type Float%20%28single-precision%29))
  (Networking|SwitchHasAuthority
    (:Authority
      (Variables|Attributes|SetHealth (- (Variables|Attributes|GetHealth) Damage))
      (if (<= (Variables|Attributes|GetHealth) 0.0)
        (CallFunction|InitHealth)
        (bind _returnvalue (UserInterface|CreateWidget "/Game/UI/Death/Game_Over_Screen.Game_Over_Screen_C"))
        (UserInterface|Viewport|AddtoViewport _returnvalue 0)
        (Variables|/Script/Engine.PlayerController|SetbShowMouseCursor (Game|GetPlayerController 0) true)
        (Game|SetGamePaused true)
        (Actor|DestroyActor)))))

(fn HasBombs
  (return (> (Variables|Attributes|GetBombCount) 0)))

(fn AttemptSpawnBomb
  (Networking|SwitchHasAuthority
    (:Authority
      (bind _hasbombsremaining (CallFunction|HasBombs))
      (if _hasbombsremaining
        (Game|SpawnActorfromClass "/Game/Blueprints/Characters/Bullets_Damage/Bullet_Asset.Bullet_Asset_C" (Math|Transform|MakeTransform (+ (* (Transformation|GetActorForwardVector) (Variables|Default|GetBombSpawnDistance)) (Transformation|GetActorLocation))) "Undefined" 0 0)
        (Variables|Attributes|SetBombCount (- (Variables|Attributes|GetBombCount) 1))))))