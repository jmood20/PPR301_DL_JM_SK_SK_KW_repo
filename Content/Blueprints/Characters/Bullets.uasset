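; Paper2D character Blueprint that fires projectiles when the Attack input is pressed.
; The press waits briefly, spawns a Bullet_Asset at the Arrow10 component's transform, then waits again, setting the Bullets flag false before and after.
; A separate Attack_Bullets event switches the flipbook to the left attack animation and halts movement, but nothing in this graph calls it.
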(event Custom|Attack_Bullets
  (Sprite|SetFlipbook (Variables|Default|GetPaperFlipbook) "/Game/Blueprints/Characters/RaspBerry_Folder/Raspberry_sprite/Left/Attack_Lerft.Attack_Lerft")
  (Components|Movement|StopMovementImmediately (Variables|Character|GetCharacterMovement)))

(event EventBeginPlay)

(event Collision|EventActorBeginOverlap
  (params (OtherActor :type Actor%20Object%20Reference)))

(event EventTick
  (params (DeltaSeconds :type Float%20%28single-precision%29)))

(event Input|ActionEvents|InputActionAttack
  (params (Key :type Key%20Structure))
  (:Pressed
    (if true
      (Variables|Default|SetBullets false)
      (Utilities|FlowControl|Delay 0.2)
      (Game|SpawnActorfromClass "/Game/Blueprints/Characters/Bullets_Damage/Bullet_Asset.Bullet_Asset_C" (Transformation|GetWorldTransform (Variables|Default|GetArrow1_0)) "Undefined" 0 0)
      (Utilities|FlowControl|Delay 0.3)
      (Variables|Default|SetBullets false))))

(fn ConstructionScript
  (|CallParentFunction))